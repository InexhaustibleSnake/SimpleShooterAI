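; Base AI controller that runs a behavior tree and registers a perceived player pawn as the enemy.
; BeginPlay starts the configured behavior tree asset.
; Perception updates pass the actor to CheckNoticedActor, which writes it to the blackboard's enemy key if it matches the player pawn class and the brain component is valid.
; The stimulus is not inspected, and the key is never cleared here.
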(event OnTargetPerceptionUpdated(AIPerceptionComponent)
  (params (Actor :type Actor%20Object%20Reference) (Stimulus :type AI%20Stimulus%20Structure))
  (CallFunction|CheckNoticedActor Actor))

(event EventBeginPlay
  (|CallParentFunction)
  (AI|RunBehaviorTree (Variables|Default|GetBTAsset)))

(fn ConstructionScript)

(fn CheckNoticedActor
  (params (Actor :type Actor%20Object%20Reference))
  (if (Class|GameplayStatics|ObjectIsA Actor (Variables|Default|GetPlayerPawnClass))
    (Utilities|IsValid (Variables|Default|GetBrainComponent)
      (:Is%20Valid
        (AI|Components|Blackboard|SetValueasObject (AI|GetBlackboard 0) (LocalVariables|GetEnemyActorKeyName) Actor)))))